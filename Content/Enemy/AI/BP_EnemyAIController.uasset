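; AI controller for patrolling enemies that runs BT_AIPatrolEnemy and reacts to sight and hearing.
; Sensing an "Enemy"-tagged actor by sight sets the player character as the Blackboard's Player key, otherwise clearing it.
; Hearing one holds Standing during the pawn's look-around, then sends hearing state and both locations to the GameInstance.
; Both senses request perception prediction; the EQS target-point query and ping-pong patrol logic are left unwired.
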(event OnTargetPerceptionUpdated(ForSightPerception)
  (params (Actor :type Actor%20Object%20Reference) (Stimulus :type AI%20Stimulus%20Structure))
  (bind _returnvalue (Utilities|String|StringToName "Player"))
  (bind _blackboard (Variables|Default|GetBlackboard))
  ;[0 1 0.1066] GoToPlayer
  (if (and (Actor|ActorHasTag Actor "Enemy") (.bSuccessfullySensed (Utilities|Struct|BreakAIStimulus Stimulus)))
    (Class|AISensePrediction|RequestControllerPredictionEvent self 0 2.0)
    (AI|Components|Blackboard|SetValueasObject _blackboard _returnvalue (Game|GetPlayerCharacter 0))
    (else
      (AI|Components|Blackboard|ClearValue _blackboard _returnvalue))))

(event OnTargetPerceptionUpdated(ForHearingPerception)
  (params (Actor :type Actor%20Object%20Reference) (Stimulus :type AI%20Stimulus%20Structure))
  (bind _bsuccessfullysensed (Utilities|Struct|BreakAIStimulus Stimulus))
  (bind _returnvalue (Actor|ActorHasTag Actor "Enemy"))
  (bind _returnvalue_2 (Game|GetGameInstance))
  (bind _returnvalue_3 (and _returnvalue _bsuccessfullysensed))
  ;[1 0.6738 0] HearAndDogChecked
  (if _returnvalue_3
    (AI|Components|Blackboard|SetValueasBool (Variables|Default|GetBlackboard) (Utilities|String|StringToName "Standing") true)
    (bind _duretiontime (Class|BPIforEnmeyControlled|StopandPlayLookAround(Message) (Pawn|GetControlledPawn)))
    (Utilities|FlowControl|Delay _duretiontime)
    (AI|Components|Blackboard|SetValueasBool (Variables|Default|GetBlackboard) (Utilities|String|StringToName "Standing") false)
    (Class|AISensePrediction|RequestControllerPredictionEvent self 0 2.0)
    (Class|BPIforGameInstance|ChangeHearingState(Message) _returnvalue_2 _returnvalue_3)
    (Class|BPIforGameInstance|GetCurrentPlayerLocation(Message) _returnvalue_2 (Transformation|GetActorLocation (Game|GetPlayerCharacter 0)))
    (Class|BPIforGameInstance|GetCurrentEnemyLocation(Message) _returnvalue_2 (Transformation|GetActorLocation (Pawn|GetControlledPawn)))))

(event Custom|SuccesQueryGo
  (params (QueryInstance :type Env%20Query%20Instance%20Blueprint%20Wrapper%20Object%20Reference) (QueryStatus :type EEnvQueryStatus%20Enum :default "Processing"))
  (bind _targetpointslist (Variables|Default|GetTargetPointsList))
  (AI|EQS|GetQueryResultsasActors QueryInstance)
  (if (Utilities|IsValid 0)
    (AI|Components|Blackboard|SetValueasObject (Variables|Default|GetBlackboard) (Utilities|String|StringToName "TargetPoints") 0)
    (Utilities|Array|Add _targetpointslist 0)
    (bind _output_get (Variables|Default|SetCurrentIndex (Utilities|Array|LastIndex _targetpointslist)))
    (AI|Components|Blackboard|SetValueasObject (Variables|Default|GetBlackboard) (Utilities|String|StringToName "TargetPoints") (Utilities|Array|Get(acopy) _targetpointslist _output_get))))

(event EventBeginPlay
  (AI|RunBehaviorTree "/Game/Enemy/AI/BT_AIPatrolEnemy.BT_AIPatrolEnemy"))

(event EventTick
  (params (DeltaSeconds :type Float%20%28single-precision%29)))

(fn ConstructionScript)