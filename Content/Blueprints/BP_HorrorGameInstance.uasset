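; Game instance for a horror game that holds shared player survival state and enemy AI state.
; Sprint start and stop swap looping timers that drain or regenerate stamina, broadcasting changes and lowering walk speed when empty.
; Also tracks HP through damage and counted medicine use.
; Stores movement, wolf speed and hearing state, returning the heard chase location or the first AI_Enemy's own position when nothing is heard.
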(event Custom|DecreaseStamina
  (bind _output_get (Variables|Default|SetStamina (Math|Float|Clamp(Float) (- (Variables|Default|GetStamina) 1e+01) 0.0 1e+02)))
  (Default|CallEDStaminaExhausting _output_get)
  (if (== _output_get 0.0)
    (Variables|/Script/Engine.CharacterMovementComponent|SetMaxWalkSpeed (Variables|/Script/Engine.Character|GetCharacterMovement (Game|GetPlayerCharacter 0)) 3e+02)))

(event Custom|IncreaseStamina
  (bind _output_get (Variables|Default|SetStamina (Math|Float|Clamp(Float) (+ (Variables|Default|GetStamina) 2e+01) 0.0 1e+02)))
  (Default|CallEDStaminaExhausting _output_get))

(event EventInit
  (Default|CallEDStaminaExhausting (Variables|Default|GetRuntime)))

(event EventUseMedicine
  (Math|Integer|DecrementInt (Variables|Default|GetMedicineCount)
    (:%20%20
      (Variables|Default|SetHP (Math|Integer|Clamp(Integer) (+ (Variables|Default|GetHP) 20) 0 100)))))

(event EventStartSprint
  (bind _returnvalue (Utilities|Time|SetTimerbyEvent (delegate Custom|DecreaseStamina) 0.5 true))
  (Variables|Default|SetStartSprinttime _returnvalue)
  (Utilities|Time|PauseTimerbyHandle (Variables|Default|GetStopsrinttime)))

(event EventChangeForwardSpeed
  (params (NewSpeed :type Integer))
  (Variables|Default|SetForwardSpeedOfWolf NewSpeed))

(event EventStopSprint
  (bind _returnvalue (Utilities|Time|SetTimerbyEvent (delegate Custom|IncreaseStamina) 0.5 true))
  (Variables|Default|SetStopsrinttime _returnvalue)
  (Utilities|Time|PauseTimerbyHandle (Variables|Default|GetStartSprinttime)))

(event EventChangeHearingState
  (params (HearingState :type Boolean))
  (Variables|Default|SetHearing HearingState))

(event EventDamageHP
  (params (Damage :type Integer))
  (bind _output_get (Variables|Default|SetHP (- (Variables|Default|GetHP) Damage)))
  (Development|PrintString (Utilities|String|ToString(Integer) _output_get)))

(event EventSetMovingState
  (params (MovingState :type Boolean))
  (Variables|Default|SetIsMoving MovingState))

(event EventGetCurrentPlayerPosition
  (params (CurrentPosition :type Vector :default "0, 0, 0"))
  (Variables|Default|SetChasingLocationFromHearing CurrentPosition))

(fn CheckMedicineCount
  (return (> (Variables|Default|GetMedicineCount) 0)))

(fn CheckStamina
  (return (> (Variables|Default|GetStamina) 0.0)))

(fn GetCharacter
  (if (Variables|Default|GetHearing)
    _
    (else
      (bind _outactors (Actor|GetAllActorsOfClass "/Game/Enemy/AI/AI_Enemy.AI_Enemy_C"))
      (Variables|Default|SetChasingLocationFromHearing (Transformation|GetActorLocation (Utilities|Array|Get(acopy) _outactors)))))
  (return (Variables|Default|GetChasingLocationFromHearing)))

(fn GetForwardSpeed
  (return (Variables|Default|GetForwardSpeedOfWolf)))

(fn IsHearing
  (return (Variables|Default|GetHearing)))

(fn IsMovingorNot
  (return (Variables|Default|GetIsMoving)))