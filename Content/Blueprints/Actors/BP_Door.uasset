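; A physics door that starts locked or free, swinging on a constraint whose Swing1 limit acts as the lock.
; A box trigger on locked doors enables F input for the player and unlocks temporarily while the Game Instance's enemy actor overlaps.
; On F, the player character reports key possession and animation time; after that delay, a key frees the door permanently and destroys the trigger.
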(event OnComponentBeginOverlap(Box)
  (params (OverlappedComponent :type Primitive%20Component%20Object%20Reference) (OtherActor :type Actor%20Object%20Reference) (OtherComp :type Primitive%20Component%20Object%20Reference) (OtherBodyIndex :type Integer) (bFromSweep :type Boolean) (SweepResult :type Hit%20Result%20Structure%20%28by%20ref%29))
  (if (== OtherActor (Game|GetPlayerCharacter 0))
    (Input|EnableInput (Game|GetPlayerController 0))
    (else
      (bind _enemy (Class|BPIforGameInstance|GetEnemyObject(Message) (Game|GetGameInstance)))
      (if (== _enemy OtherActor)
        (Variables|Default|SetLocked false)
        (Class|PhysicsConstraintComponent|SetAngularSwing1Limit (Variables|Default|GetPhysicsConstraint) "ACM_Free" 9e+01)))))

(event OnComponentEndOverlap(Box)
  (params (OverlappedComponent :type Primitive%20Component%20Object%20Reference) (OtherActor :type Actor%20Object%20Reference) (OtherComp :type Primitive%20Component%20Object%20Reference) (OtherBodyIndex :type Integer))
  (if (== OtherActor (Game|GetPlayerCharacter 0))
    (Input|DisableInput (Game|GetPlayerController 0))
    (else
      (bind _enemy (Class|BPIforGameInstance|GetEnemyObject(Message) (Game|GetGameInstance)))
      (if (== _enemy OtherActor)
        (Variables|Default|SetLocked true)
        (Class|PhysicsConstraintComponent|SetAngularSwing1Limit (Variables|Default|GetPhysicsConstraint) "ACM_Limited" 0.0)))))

(event EventBeginPlay
  (bind _physicsconstraint (Variables|Default|GetPhysicsConstraint))
  (if (Variables|Default|GetLocked)
    (Class|PhysicsConstraintComponent|SetAngularSwing1Limit _physicsconstraint "ACM_Limited" 0.0)
    (else
      (Class|PhysicsConstraintComponent|SetAngularSwing1Limit _physicsconstraint "ACM_Free" 9e+01)
      (Components|DestroyComponent (Variables|Default|GetBox)))))

(event Collision|EventActorBeginOverlap
  (params (OtherActor :type Actor%20Object%20Reference)))

(event EventTick
  (params (DeltaSeconds :type Float%20%28single-precision%29)))

(event Input|KeyboardEvents|F
  (params (Key :type Key%20Structure :default "None"))
  (:Pressed
    (bind (_havekey _animationtime) (Class|BPIOpenDoor|OpenDoor(Message) (Game|GetPlayerCharacter 0)))
    (Utilities|FlowControl|Delay _animationtime)
    (if _havekey
      (Class|PhysicsConstraintComponent|SetAngularSwing1Limit (Variables|Default|GetPhysicsConstraint) "ACM_Free" 9e+01)
      (Components|DestroyComponent (Variables|Default|GetBox)))))

(fn ConstructionScript)