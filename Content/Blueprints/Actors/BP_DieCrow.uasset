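; BP_DieCrow is a one-shot trigger actor that cues a falling crow when the player character enters its box.
; On overlap it turns on the game instance's moving-state flag through a message call and immediately sends the falling message to the referenced Crow.
; After a three-second delay it turns the flag off and destroys itself.
; A PlayMontage node is left unconnected.
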(event OnComponentBeginOverlap(Box)
  (params (OverlappedComponent :type Primitive%20Component%20Object%20Reference) (OtherActor :type Actor%20Object%20Reference) (OtherComp :type Primitive%20Component%20Object%20Reference) (OtherBodyIndex :type Integer) (bFromSweep :type Boolean) (SweepResult :type Hit%20Result%20Structure%20%28by%20ref%29))
  (bind _returnvalue (Game|GetPlayerCharacter 0))
  (bind _returnvalue_2 (Game|GetGameInstance))
  (bind _returnvalue_3 (== OtherActor _returnvalue))
  (if _returnvalue_3
    (Utilities|FlowControl|Sequence
      (:then_0
        (Class|BPIforGameInstance|SetMovingState(Message) _returnvalue_2 true)
        (Utilities|FlowControl|Delay 3.0)
        (Class|BPIforGameInstance|SetMovingState(Message) _returnvalue_2 false)
        (Actor|DestroyActor))
      (:then_1
        (Class|BPIDeathCrow|IsFallingCrow(Message) (Variables|Default|GetCrow) _returnvalue_3)))))

(event EventBeginPlay)

(event Collision|EventActorBeginOverlap
  (params (OtherActor :type Actor%20Object%20Reference)))

(event EventTick
  (params (DeltaSeconds :type Float%20%28single-precision%29)))

(fn ConstructionScript)