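; Game instance for a horror game that holds player stamina, HP, medicine count and moving state, with query functions.
; Sprint start and stop create looping timers that drain or refill stamina, each pausing the opposite timer.
; Stamina changes broadcast through an event dispatcher, clamped only for output, and exhaustion lowers the player's walk speed.
; Medicine restores clamped HP, while damage subtracts unclamped and prints the result.
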(event Custom|DecreaseStamina
  (bind _output_get (Variables|Default|SetStamina (- (Variables|Default|GetStamina) 1e+01)))
  (Default|CallEDStaminaExhausting (Math|Float|Clamp(Float) _output_get 0.0 1e+02))
  (if (== (Math|Float|Clamp(Float) _output_get 0.0 1e+02) 0.0)
    (Variables|/Script/Engine.CharacterMovementComponent|SetMaxWalkSpeed (Variables|/Script/Engine.Character|GetCharacterMovement (Game|GetPlayerCharacter 0)) 3e+02)))

(event Custom|IncreaseStamina
  (bind _output_get (Variables|Default|SetStamina (+ (Variables|Default|GetStamina) 2e+01)))
  (Default|CallEDStaminaExhausting (Math|Float|Clamp(Float) _output_get 0.0 1e+02)))

(event EventInit
  (Default|CallEDStaminaExhausting (Variables|Default|GetRuntime)))

(event EventUseMedicine
  (Math|Integer|DecrementInt (Variables|Default|GetMedicineCount)
    (:%20%20
      (Variables|Default|SetHP (Math|Integer|Clamp(Integer) (+ (Variables|Default|GetHP) 20) 0 100)))))

(event EventStartSprint
  (bind _returnvalue (Utilities|Time|SetTimerbyEvent (delegate Custom|DecreaseStamina) 0.5 true))
  (Variables|Default|SetStartSprinttime _returnvalue)
  (Utilities|Time|PauseTimerbyHandle (Variables|Default|GetStopsrinttime)))

(event EventStopSprint
  (bind _returnvalue (Utilities|Time|SetTimerbyEvent (delegate Custom|IncreaseStamina) 0.5 true))
  (Variables|Default|SetStopsrinttime _returnvalue)
  (Utilities|Time|PauseTimerbyHandle (Variables|Default|GetStartSprinttime)))

(event EventDamageHP
  (params (Damage :type Integer))
  (bind _output_get (Variables|Default|SetHP (- (Variables|Default|GetHP) Damage)))
  (Development|PrintString (Utilities|String|ToString(Integer) _output_get)))

(event EventSetMovingState
  (params (MovingState :type Boolean))
  (Variables|Default|SetIsMoving MovingState))

(fn CheckMedicineCount
  (return (> (Variables|Default|GetMedicineCount) 0)))

(fn CheckStamina
  (return (> (Variables|Default|GetStamina) 0.0)))

(fn IsMovingorNot
  (return (Variables|Default|GetIsMoving)))