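; Physics-driven swinging door that can start locked and be unlocked by a player who has a key.
; When locked, a physics constraint holds the swing at zero; otherwise the swing is free and the trigger Box is destroyed at BeginPlay.
; Overlapping actors implementing BPI_OpenDoor toggle the door's input on entering and leaving the Box.
; Pressing F calls OpenDoorMessage on the player character, waits the returned animation time, then frees the door and removes the Box if HaveKey is true.
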(event OnComponentBeginOverlap(Box)
  (params (OverlappedComponent :type Primitive%20Component%20Object%20Reference) (OtherActor :type Actor%20Object%20Reference) (OtherComp :type Primitive%20Component%20Object%20Reference) (OtherBodyIndex :type Integer) (bFromSweep :type Boolean) (SweepResult :type Hit%20Result%20Structure%20%28by%20ref%29))
  (if (Utilities|DoesObjectImplementInterface OtherActor "/Game/FirstPartGame/Blueprints/InterFaces/ForImplement/BPI_OpenDoor.BPI_OpenDoor_C")
    (Input|EnableInput (Game|GetPlayerController 0))))

(event OnComponentEndOverlap(Box)
  (params (OverlappedComponent :type Primitive%20Component%20Object%20Reference) (OtherActor :type Actor%20Object%20Reference) (OtherComp :type Primitive%20Component%20Object%20Reference) (OtherBodyIndex :type Integer))
  (if (Utilities|DoesObjectImplementInterface OtherActor "/Game/FirstPartGame/Blueprints/InterFaces/ForImplement/BPI_OpenDoor.BPI_OpenDoor_C")
    (Input|DisableInput (Game|GetPlayerController 0))))

(event EventBeginPlay
  (bind _physicsconstraint (Variables|Default|GetPhysicsConstraint))
  (if (Variables|Default|GetLocked)
    (Class|PhysicsConstraintComponent|SetAngularSwing1Limit _physicsconstraint "ACM_Limited" 0.0)
    (else
      (Class|PhysicsConstraintComponent|SetAngularSwing1Limit _physicsconstraint "ACM_Free" 9e+01)
      (Components|DestroyComponent (Variables|Default|GetBox)))))

(event Collision|EventActorBeginOverlap
  (params (OtherActor :type Actor%20Object%20Reference)))

(event EventTick
  (params (DeltaSeconds :type Float%20%28single-precision%29)))

(event Input|KeyboardEvents|F
  (params (Key :type Key%20Structure :default "None"))
  (:Pressed
    (bind (_havekey _animationtime) (Class|BPIOpenDoor|OpenDoor(Message) (Game|GetPlayerCharacter 0)))
    (Utilities|FlowControl|Delay _animationtime)
    (if _havekey
      (Class|PhysicsConstraintComponent|SetAngularSwing1Limit (Variables|Default|GetPhysicsConstraint) "ACM_Free" 9e+01)
      (Components|DestroyComponent (Variables|Default|GetBox)))))

(fn ConstructionScript)