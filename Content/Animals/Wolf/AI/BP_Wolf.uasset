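; BP_Wolf is a wolf Blueprint whose only implemented logic is a function that computes a desired movement vector.
; WolfDesiredMovement builds forward and right vectors from control yaw alone and scales them by movement inputs, doubling the sum when Running.
; The axes are crossed: the forward vector uses MoveRight and the right vector uses MoveForward.
; The event graph and construction script are empty.
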(event EventBeginPlay)

(event Collision|EventActorBeginOverlap
  (params (OtherActor :type Actor%20Object%20Reference)))

(event EventTick
  (params (DeltaSeconds :type Float%20%28single-precision%29)))

(fn ConstructionScript)

(fn WolfDesiredMovement
  (bind _returnvalue (Pawn|GetControlRotation :!class /Script/Engine.Pawn))
  (return (* (+ (* (Math|Vector|GetForwardVector (Math|Rotator|MakeRotator 0.0 0.0 (.yaw _returnvalue))) (Input|AxisValues|GetMoveRight)) (* (Math|Vector|GetRightVector (Math|Rotator|MakeRotator 0.0 0.0 (.yaw _returnvalue))) (Input|AxisValues|GetMoveForward))) (Math|Float|SelectFloat 2.0 1.0 (Variables|Default|GetRunning)))))