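; BP_Crocodile is the crocodile animal character, holding target state and patrol-style target points, likely for its AI to use.
; An event sets the InTarget flag, and getter functions return that flag and the PointTargets variable.
; Another event plays a slowed left walk-turn root-motion montage and stops it after a short delay, producing a brief partial turn.
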(event EventInTargetorNot
  (params (CheckTarget :type Boolean))
  (Variables|Default|SetInTarget? CheckTarget))

(event EventPlayCrocodileAnimMontage
  (Animation|PlayAnimMontage "/Game/Animals/Crocodile/Animations/ANIM_Crocodile_WalkTurnL_RM_Montage.ANIM_Crocodile_WalkTurnL_RM_Montage" 0.4 "None")
  (Utilities|FlowControl|Delay 0.25)
  (Animation|StopAnimMontage "/Game/Animals/Crocodile/Animations/ANIM_Crocodile_WalkTurnL_RM_Montage.ANIM_Crocodile_WalkTurnL_RM_Montage"))

(event EventBeginPlay)

(fn ConstructionScript)

(fn IsinTarget
  (return (Variables|Default|GetInTarget?)))

(fn TargetPoints
  (return (Variables|Default|GetPointTargets)))